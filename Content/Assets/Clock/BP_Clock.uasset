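; BP_Clock is a clock actor whose hour, minute and second hands show a time stored in integer variables.
; The Construction Script poses the hands through SetUpHands, converting each value to a roll angle and folding hours above 12 onto the dial.
; If IsFunctional is set at BeginPlay, a one-second Delay loop runs ClockLogic, which advances the 24-hour time with rollover and re-poses the hands in discrete steps.
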(event Custom|SetUpHands
  (CallFunction|HoursSetUp)
  (CallFunction|MinutesSetUp)
  (CallFunction|SecondsSetUp))

(event EventBeginPlay
  (if (Variables|Default|GetIs%20functional)
    (Utilities|FlowControl|Delay 1.0 :!label _label)
    (CallFunction|ClockLogic)
    (goto _label)))

(event Collision|EventActorBeginOverlap
  (params (OtherActor :type Actor%20Object%20Reference)))

(event EventTick
  (params (DeltaSeconds :type Float%20%28single-precision%29)))

(fn ConstructionScript
  (CallFunction|SetUpHands))

(fn HoursSetUp
  (bind _clock_hours (Variables|Default|GetClock_hours))
  (bind _hours (Variables|Default|GetHours))
  (Math|Integer|CompareInt _hours 12
    (:>
      (bind _result (Utilities|NegateInt (* (/ 360 12) (- (Variables|Default|GetHours) 12)))
        (:%20%20
          (Transformation|SetRelativeRotation _clock_hours (Math|Rotator|MakeRotator (Math|Conversions|ToFloat(Integer) _result) 0.0 0.0) false false))))
    (:==
      (bind _result_2 (Utilities|NegateInt (* _hours (/ 360 12)) :!label _label)
        (:%20%20
          (Transformation|SetRelativeRotation _clock_hours (Math|Rotator|MakeRotator (Math|Conversions|ToFloat(Integer) _result_2) 0.0 0.0) false false))))
    (:<
      (goto _label))))

(fn MinutesSetUp
  (bind _result (Utilities|NegateInt (* (Variables|Default|GetMinutes) (/ 360 60)))
    (:%20%20
      (Transformation|SetRelativeRotation (Variables|Default|GetClock_minutes) (Math|Rotator|MakeRotator (Math|Conversions|ToFloat(Integer) _result) 0.0 0.0) false false))))

(fn SecondsSetUp
  (bind _result (Utilities|NegateInt (* (Variables|Default|GetSeconds) (/ 360 60)))
    (:%20%20
      (Transformation|SetRelativeRotation (Variables|Default|GetClock_seconds) (Math|Rotator|MakeRotator (Math|Conversions|ToFloat(Integer) _result) 0.0 0.0) false false))))

(fn ClockLogic
  (Math|Integer|CompareInt (Variables|Default|GetSeconds) 59
    (:>
      (Variables|Default|SetSeconds 0 :!label _label)
      (Math|Integer|CompareInt (Variables|Default|GetMinutes) 59
        (:>
          (Variables|Default|SetMinutes 0 :!label _label_2)
          (Math|Integer|CompareInt (Variables|Default|GetHours) 23
            (:>
              (Variables|Default|SetHours 0 :!label _label_3))
            (:==
              (goto _label_3))
            (:<
              (Math|Integer|IncrementInt (Variables|Default|GetHours)
                (:%20%20
                  _)))))
        (:==
          (goto _label_2))
        (:<
          (Math|Integer|IncrementInt (Variables|Default|GetMinutes)
            (:%20%20
              _)))))
    (:==
      (goto _label))
    (:<
      (Math|Integer|IncrementInt (Variables|Default|GetSeconds)
        (:%20%20
          _))))
  (CallFunction|SetUpHands)
  (return))