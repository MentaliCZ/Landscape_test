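; Crow-specific AI actor that extends its parent's state and death handling with animation, flight sound and a corpse.
; State changes call the parent, then clear the crow AnimBP's on-ground flag and start the flight sound for one enum state, apparently flight.
; A separate function stops the sound component only if the flight sound is assigned.
; Death spawns a crow corpse slightly below the actor before calling the parent death.
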(fn ConstructionScript)

(fn Death
  (bind _returnvalue (Transformation|GetActorTransform))
  (bind _self self)
  (bind (_location _rotation _scale) (Math|Transform|BreakTransform _returnvalue))
  (bind (_x _y _z) (Math|Vector|BreakVector _location))
  (Game|SpawnActorfromClass "/Game/Actors/blueprints/crow/CrowCorpse.CrowCorpse_C" (Math|Transform|MakeTransform (Math|Vector|MakeVector _x _y (+ _z -75.0)) _rotation _scale) "Undefined" _self _self)
  (|CallParentFunction))

(fn ChangeState
  (params (state :type AIStateEnum%20Enum :default "NewEnumerator0"))
  (bind _returnvalue (Utilities|Enum|Equal(Enum) state "NewEnumerator8"))
  (|CallParentFunction state)
  (bind _asbpa_crow (Utilities|Casting|CastToBPA_Crow (Components|SkeletalMesh|GetAnimInstance (Variables|Character|GetMesh))))
  (Variables|/Game/Actors/blueprints/crow/BPA_Crow.BPA_Crow_C|SetisOnGround _asbpa_crow (not _returnvalue))
  (if _returnvalue
    (CallFunction|PlayFlightSound)))

(fn PlayFlightSound
  (bind _soundcomponent (Variables|Default|GetsoundComponent))
  (if (not (Audio|Components|Audio|IsPlaying _soundcomponent))
    (Audio|Components|Audio|SetSound _soundcomponent (Variables|Default|GetflightSound))
    (Audio|Components|Audio|Play _soundcomponent 0.0)))

(fn StopFlightSound
  (bind _soundcomponent (Variables|Default|GetsoundComponent))
  (if (== (Variables|/Script/Engine.AudioComponent|GetSound _soundcomponent) (Variables|Default|GetflightSound))
    (Audio|Components|Audio|Stop _soundcomponent)))