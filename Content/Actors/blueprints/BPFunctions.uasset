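; Blueprint function library of helpers for finding the nearest actor by class and testing class membership.
; GetClosestActor linearly scans all actors of a class for the smallest distance to the caller.
; GetClosestOfClasses runs that search per class and keeps the nearest valid result.
; IsOfClass matches equal or child classes, while IsOfClassArray loops over a list but leaves the child check's TestClass unset.
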(fn GetClosestActor
  (params (caller :type Actor%20Object%20Reference) (class :type Actor%20Class%20Reference))
  (LocalVariables|SetLowest%20dist 1e+10)
  (bind _outactors (Actor|GetAllActorsOfClass caller class))
  (for _array_element _outactors
    (Math|Float|CompareFloat (Math|Vector|Distance(Vector) (Transformation|GetActorLocation _array_element) (Transformation|GetActorLocation caller)) (LocalVariables|GetLowest%20dist)
      (:<
        (LocalVariables|SetLowest%20dist (Math|Vector|Distance(Vector) (Transformation|GetActorLocation _array_element) (Transformation|GetActorLocation caller)))
        (LocalVariables|Setclosest _array_element))))
  (return (LocalVariables|Getclosest)))

(fn IsOfClass
  (params (actor :type Actor%20Class%20Reference) (class :type Actor%20Class%20Reference))
  (return (or (== actor class) (Utilities|ClassIsChildOf actor class))))

(fn IsOfClassArray
  (params (classes :type Array%20of%20Actor%20Class%20References) (actor :type Actor%20Class%20Reference))
  (bind _array_element (Utilities|Array|ForEachLoopwithBreak classes)
    (:LoopBody
      (if (or (== actor _array_element) (Utilities|ClassIsChildOf 0 _array_element))
        (return true)))
    (:Completed
      (return false))))

(fn GetClosestOfClasses
  (params (caller :type Actor%20Object%20Reference) (class :type Array%20of%20Actor%20Class%20References) (__WorldContext :type Object%20Object%20Reference))
  (LocalVariables|Setclosest 0)
  (LocalVariables|SetLowest%20dist 1e+10)
  (for _array_element class
    (bind _closestactor (CallFunction|GetClosestActor caller _array_element __WorldContext))
    (Utilities|IsValid _closestactor
      (:Is%20Valid
        (Math|Float|CompareFloat (Math|Vector|Distance(Vector) (Transformation|GetActorLocation _closestactor) (Transformation|GetActorLocation caller)) (LocalVariables|GetLowest%20dist)
          (:<
            (LocalVariables|SetLowest%20dist (Math|Vector|Distance(Vector) (Transformation|GetActorLocation _closestactor) (Transformation|GetActorLocation caller)))
            (LocalVariables|Setclosest _closestactor))))))
  (return (LocalVariables|Getclosest)))