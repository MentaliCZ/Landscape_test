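; AI controller for animals that runs a passive behavior tree and flees perceived threats.
; IsScary flags feared classes, optionally the player, threats same-species animals recently fled, and is meant to catch predators attacking its species.
; Threats set target and mode on the controller and blackboard, and can be learned as feared classes.
; Non-threatening perception updates start a repeating timer check that clears targets once invalid or far enough away.
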(event OnTargetPerceptionUpdated(AIPerception)
  (params (Actor :type Actor%20Object%20Reference) (Stimulus :type AI%20Stimulus%20Structure))
  ;[1 1 1] Detect scary targets
  (bind (_is_ _target) (CallFunction|IsScary Actor))
  (if (and _is_ (.bSuccessfullySensed (Utilities|Struct|BreakAIStimulus Stimulus)))
    (CallFunction|SetTarget _target "NewEnumerator0")
    ;[1 1 1] This animal has just learnt about new potential threat.
    (if (Variables|Default|GetcanLearn)
      (Utilities|Array|AddUnique (Variables|Default|GetafraidOf) (Utilities|GetClass _target)))
    (else
      (Utilities|Time|SetTimerbyEvent (delegate Custom|AIReset) 1e+01))))

(event Custom|AIReset
  (bind _currenttarget (Variables|Default|GetcurrentTarget))
  ;[1 1 1] Target reset if distant
  (Utilities|IsValid _currenttarget
    (:Is%20Valid
      (switch Utilities|FlowControl|Switch|SwitchonAITargetModeEnum (Variables|Default|GettargetMode)
        (:NewEnumerator2
          (CallFunction|ResetTarget :!label _label))
        (:NewEnumerator0
          (if (> (Math|Vector|Distance(Vector) (Transformation|GetActorLocation _currenttarget) (Transformation|GetActorLocation (Pawn|GetControlledPawn))) (Variables|Default|GetdistanceToLooseTarget)) :!label _label_2
            (goto _label)
            (else
              (Utilities|Time|SetTimerbyEvent (delegate Custom|AIReset) 1e+01))))
        (:NewEnumerator1
          (goto _label_2))))
    (:Is%20Not%20Valid
      (CallFunction|ResetTarget))))

(event Custom|OnTargetReset)

(event EventPossess
  (params (PossessedPawn :type Pawn%20Object%20Reference))
  (AI|RunBehaviorTree "/Game/Actors/blueprints/ai/BT_Animal_Passive.BT_Animal_Passive"))

(fn ConstructionScript)

(fn IsScary
  (params (actor :type Actor%20Object%20Reference))
  (bind _self self)
  (bind _returnvalue (Pawn|GetControlledPawn _self))
  (bind _returnvalue_2 (Utilities|GetClass _returnvalue))
  ;[1 1 1] Check Ignored or Auto positive
  (bind _output_get (LocalVariables|SetcheckedActor actor))
  (bind _result (CallFunction|IsOfClassArray (Variables|Default|GetafraidOf) (Utilities|GetClass _output_get)))
  (if _result
    (Variables|Default|SetlastSeenTarget (Utilities|Time|GetGameTimeinSeconds))
    (return true (LocalVariables|GetcheckedActor))
    (else
      (bind _result_2 (CallFunction|IsOfClassArray (Variables|Default|Getignored) (Utilities|GetClass _output_get)))
      (if _result_2
        (return false 0)
        (else
          (bind _asanimal_master_ai (Utilities|Casting|CastToAnimalMasterAI (LocalVariables|GetcheckedActor))
            (:then
              (bind _asanimal_aicontroller (Utilities|Casting|CastToAnimalAIController (AI|GetAIController _asanimal_master_ai))
                (:then
                  (bind _result_3 (CallFunction|IsOfClass (Utilities|GetClass _asanimal_master_ai) _returnvalue_2))
                  (if _result_3
                    ;[1 1 1] Is a member of the same species afraid of something?
                    (switch Utilities|FlowControl|Switch|SwitchonAITargetModeEnum (Variables|AnimalAIController_C|GettargetMode _asanimal_aicontroller)
                      (:NewEnumerator2
                        _)
                      (:NewEnumerator0
                        (if (> (Variables|AnimalAIController_C|GetlastSeenTarget _asanimal_aicontroller) (Variables|Default|GetlastSeenTarget))
                          (Variables|Default|SetlastSeenTarget (Variables|AnimalAIController_C|GetlastSeenTarget _asanimal_aicontroller))
                          (return true (Variables|AnimalAIController_C|GetcurrentTarget _asanimal_aicontroller))
                          (else
                            _)))
                      (:NewEnumerator1
                        _))
                    (return false 0)
                    (else
                      ;[1 1 1] Is a member of the same species being attacked by this
                      (switch Utilities|FlowControl|Switch|SwitchonAITargetModeEnum (Variables|AnimalAIController_C|GettargetMode _asanimal_aicontroller)
                        (:NewEnumerator2
                          _)
                        (:NewEnumerator0
                          _)
                        (:NewEnumerator1
                          (bind _asactor (Utilities|Casting|CastToActorClass (Utilities|GetClass (Variables|AnimalAIController_C|GetcurrentTarget _asanimal_aicontroller)))
                            (:then
                              (bind _result_4 (CallFunction|IsOfClass _asactor _returnvalue_2))
                              (if _result_4
                                (Variables|Default|SetlastSeenTarget (Utilities|Time|GetGameTimeinSeconds)))
                              (return _result_4 (LocalVariables|GetcheckedActor)))
                            (:CastFailed
                              (return false 0)))))
                      (return false 0))))
                (:CastFailed
                  (return false 0))))
            (:CastFailed
              (return (and (Actor|ActorHasTag (LocalVariables|GetcheckedActor) "Player") (Variables|Default|GetafraidOfPlayer)) (LocalVariables|GetcheckedActor)))))))))

(fn SetTarget
  (params (actor :type Actor%20Object%20Reference) (mode :type AITargetModeEnum%20Enum :default "NewEnumerator2"))
  (bind _blackboard (Variables|Default|GetBlackboard))
  (AI|Components|Blackboard|SetValueasObject _blackboard (Variables|Default|GetbbTarget) actor)
  (AI|Components|Blackboard|SetValueasEnum _blackboard (Variables|Default|GetbbTargetMode) mode)
  (AI|Components|Blackboard|SetValueasBool _blackboard (Variables|Default|GetbbIsAfraid) (Utilities|Enum|Equal(Enum) mode "NewEnumerator0"))
  (AI|Components|Blackboard|SetValueasBool _blackboard (Variables|Default|Getbb%20Is%20hunting) (or (Utilities|Enum|Equal(Enum) mode "NewEnumerator1") (Utilities|Enum|Equal(Enum) mode "NewEnumerator3")))
  (Variables|Default|SettargetMode mode)
  (Variables|Default|SetcurrentTarget actor))

(fn ResetTarget
  (bind _blackboard (Variables|Default|GetBlackboard))
  (bind _blackboard_2 (Variables|Default|GetBlackboard))
  (AI|Components|Blackboard|SetValueasBool _blackboard (Variables|Default|GetbbIsAfraid) false)
  (AI|Components|Blackboard|ClearValue _blackboard (Variables|Default|GetbbTarget))
  (bind _output_get (Variables|Default|SettargetMode "NewEnumerator2"))
  (AI|Components|Blackboard|SetValueasBool _blackboard_2 (Variables|Default|Getbb%20Is%20hunting) false)
  (AI|Components|Blackboard|SetValueasEnum _blackboard_2 (Variables|Default|GetbbTargetMode) _output_get)
  (CallFunction|OnTargetReset))