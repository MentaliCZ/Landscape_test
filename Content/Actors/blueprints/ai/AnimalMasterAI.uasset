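; Base animal AI character with health, hunger and energy, plus a camera-facing debug status text.
; Its state sets movement speed and idle sound, while UpdateNeeds drains energy, applies starvation damage and reports needs to its caller.
; Montage notifies trigger capsule-overlap attacks on other animals, reporting success back to the calling object.
; Damage can cause timeline-driven speed staggers, sets the attacker as the AnimalAIController's target, or leads to delayed death.
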(event Custom|DelayedDeath
  (Utilities|FlowControl|Delay 0.3)
  (CallFunction|Death))

(event Custom|AttackEvent
  (params (montage :type Anim%20Montage%20Object%20Reference))
  (bind _soundcomponent (Variables|Default|GetsoundComponent))
  ;[1 1 1] Attack animation
  (Animation|Montage|PlayMontage (Variables|Character|GetMesh) montage 1.0 0.0 "Default"
    (:OnCompleted
      (Default|NotifyBoolean (Variables|Default|GetattackCaller) (Variables|Default|GetattackSuccess)))
    (:OnNotifyBegin
      (CallFunction|Attack)
      (Audio|Components|Audio|SetSound _soundcomponent (Variables|Default|GetattackSound))
      (Audio|Components|Audio|Play _soundcomponent 0.0))))

(event Custom|updateStatus
  ;[1 1 1] Status text update
  (Rendering|SetVisibility (Variables|Default|GetTextRender) (Variables|Default|GetshowDebugMessage) true)
  (Rendering|Components|TextRender|SetText (Variables|Default|GetTextRender) (Utilities|Text|FormatText "Health: {health} %<br>Satiety: {hng} %<br>Energy: {eng}%<br>State:{st}" (Math|Integer|Max(Integer) (Variables|Default|GetHealth)) (Math|Integer|Max(Integer) (- 100 (Math|Float|Truncate (Variables|Default|GetHunger)))) (Math|Integer|Max(Integer) (Math|Float|Truncate (Variables|Default|GetEnergy))) (Utilities|String|EnumtoString (Variables|Default|GetCurrentAIState)))))

(event Custom|HurtEvent
  (params (Montage :type Anim%20Montage%20Object%20Reference))
  (bind _soundcomponent (Variables|Default|GetsoundComponent))
  ;[1 1 1] Hurt animation
  (Animation|Montage|PlayMontage (Variables|Character|GetMesh) Montage 1.0 0.0 "Default"
    (:then
      (bind _speedmod (Timeline|Timeline_0 Play)
        (:Update
          (Variables|Default|SetrunningSpeed (* (Variables|Default|GetdefaultRunningSpeed) _speedmod))
          (Variables|Default|SetwalkingSpeed (* (Variables|Default|GetdefaultWalkingSpeed) _speedmod))
          (CallFunction|UpdateMovementSpeed))))
    (:OnNotifyBegin
      (Audio|Components|Audio|SetSound _soundcomponent (Variables|Default|GethurtSound))
      (Audio|Components|Audio|Play _soundcomponent 0.0))))

(event Custom|OnStateChange
  ;[1 1 1] State update event
  (CallFunction|UpdateMovementSpeed)
  (switch Utilities|FlowControl|Switch|SwitchonAIStateEnum (Variables|Default|GetCurrentAIState)
    (:NewEnumerator0
      (CallFunction|StopIdleSound :!label _label))
    (:NewEnumerator1
      (goto _label))
    (:NewEnumerator2
      (CallFunction|PlayIdleSound))
    (:NewEnumerator4
      (goto _label))
    (:NewEnumerator5
      (goto _label))
    (:NewEnumerator7
      (goto _label))
    (:NewEnumerator8
      (goto _label))))

(event EventTick
  (params (DeltaSeconds :type Float%20%28single-precision%29))
  ;[1 1 1] Text billboard rotation update
  (Transformation|SetWorldRotation (Variables|Default|GetTextRender) (Math|Rotator|FindLookatRotation (+ (Class|CharacterMovementComponent|GetLastUpdateLocation (Variables|Character|GetCharacterMovement)) "0, 0,40.000000") (Camera|GetCameraLocation (Game|GetPlayerCameraManager 0))) false true))

(fn ConstructionScript)

(fn ChangeState
  (params (state :type AIStateEnum%20Enum :default "NewEnumerator0"))
  (Variables|Default|SetCurrentAIState state)
  (CallFunction|OnStateChange))

(fn Hurt
  (params (damage :type Integer) (source :type Actor%20Object%20Reference))
  (bind _output_get (Variables|Default|SetHealth (- (Variables|Default|GetHealth) damage)))
  (if (< _output_get 0)
    (CallFunction|DelayedDeath)
    (return true)
    (else
      (CallFunction|HurtStagger damage)
      (CallFunction|UpdateStatus)
      (if (!= source self)
        (CallFunction|Scare source)
        (return false)
        (else
          (return false))))))

(fn Scare
  (params (source :type Actor%20Object%20Reference))
  (Utilities|IsValid source
    (:Is%20Valid
      (bind _asanimal_aicontroller (Utilities|Casting|CastToAnimalAIController (Pawn|GetController self)))
      (Default|SetTarget _asanimal_aicontroller source "NewEnumerator0"))))

(fn HurtStagger
  (params (damage :type Integer))
  ;[1 1 1] Stagger treshold
  (if (> damage (Variables|Default|GethurtDamageTreshold))
    (CallFunction|HurtEvent (Variables|Default|GethurtMontage))))

(fn Death
  (Audio|PlaySoundatLocation (Variables|Default|GetdeathSound) (Transformation|GetWorldLocation (Variables|Character|GetMesh)) "0, 0, 0" 1.0 1.0 0.0 0 0 0 0)
  (bind _asanimal_aicontroller (Utilities|Casting|CastToAnimalAIController (Pawn|GetController)))
  (Pawn|UnPossess _asanimal_aicontroller)
  (Actor|DestroyActor))

(fn AttackStart
  (params (caller :type BPI%20Callback%20Interface))
  (Variables|Default|SetattackCaller caller)
  (CallFunction|AttackEvent (Variables|Default|GetattackMontage))
  (Variables|Default|SetattackSuccess false))

(fn Attack
  (bind _self self)
  (bind _outactors (Collision|CapsuleOverlapActors (Transformation|GetWorldLocation (Variables|Default|GetAttackRange)) 1.2e+02 1e+02 (Utilities|Array|MakeArray "ObjectTypeQuery3") 0))
  (for _array_element _outactors
    (bind _asanimal_master_ai (Utilities|Casting|CastToAnimalMasterAI _array_element))
    (if (!= _asanimal_master_ai _self)
      (bind _killed (CallFunction|Hurt _asanimal_master_ai (Variables|Default|Getdamage) _self))
      (if _killed
        (Variables|Default|SetattackSuccess true)))))

(fn UpdateMovementSpeed
  (switch Utilities|FlowControl|Switch|SwitchonAIStateEnum (Variables|Default|GetCurrentAIState)
    (:NewEnumerator0
      (Variables|/Script/Engine.CharacterMovementComponent|SetMaxWalkSpeed (Variables|Character|GetCharacterMovement) (Variables|Default|GetwalkingSpeed) :!label _label))
    (:NewEnumerator1
      (goto _label))
    (:NewEnumerator2
      (goto _label))
    (:NewEnumerator4
      (Variables|/Script/Engine.CharacterMovementComponent|SetMaxWalkSpeed (Variables|Character|GetCharacterMovement) (Variables|Default|GetrunningSpeed) :!label _label_2))
    (:NewEnumerator5
      (goto _label_2))))

(fn PlayIdleSound
  (bind _soundcomponent (Variables|Default|GetsoundComponent))
  (if (not (Audio|Components|Audio|IsPlaying _soundcomponent))
    (Audio|Components|Audio|SetSound _soundcomponent (Variables|Default|GetidleSound))
    (Audio|Components|Audio|Play _soundcomponent 0.0)))

(fn StopIdleSound
  (bind _soundcomponent (Variables|Default|GetsoundComponent))
  (if (== (Variables|/Script/Engine.AudioComponent|GetSound _soundcomponent) (Variables|Default|GetidleSound))
    (Audio|Components|Audio|Stop _soundcomponent)))

(fn UpdateNeeds
  (Utilities|FlowControl|Sequence
    (:then_0
      (bind _output_get (Variables|AnimalMasterAI_C|SetEnergy self (- (Variables|Default|GetEnergy) (Variables|Default|GetenergyRate)))))
    (:then_1
      (bind _output_get_2 (Variables|Default|SetHunger (+ (Variables|Default|GetHunger) (Variables|Default|GethungerRate)))))
    (:then_2
      (if (>= _output_get_2 99.0)
        (bind _killed (CallFunction|Hurt 1))
        (LocalVariables|Setkilled _killed)))
    (:then_3
      (if (LocalVariables|Getkilled)
        (return true false false 0.0)
        (else
          (CallFunction|UpdateStatus)
          (return (LocalVariables|Getkilled) (< _output_get (Variables|Default|GetenergyTreshold)) (>= _output_get_2 (Variables|Default|GethungerTreshold)) (Variables|Default|GetHunger)))))))