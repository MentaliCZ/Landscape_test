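; Interactable container actor that the player opens with a trace hit and then loots.
; The construction script applies the configurable skeletal container mesh and the static mesh of the item inside.
; A hit on a closed container prints locked text or, if unlocked, plays the opening animation once and marks it open after one second.
; Later hits trigger the player pickup, print interaction text and destroy the item component.
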(event EventBeginPlay
  (|CallParentFunction) ; This node is disabled and will not be called.\nDrag off pins to build functionality.
)

(event EventTraceLineHit
  (params (Hit%20Component :type Actor%20Component%20Object%20Reference))
  (if (Variables|Default|GetIs%20open)
    (CallFunction|PickupContainerItem)
    (else
      (bind _isunlocked (CallFunction|IsUnlocked))
      (if _isunlocked
        (Utilities|FlowControl|DoOnce false
          (:Completed
            (CallFunction|Interaction)
            (Utilities|FlowControl|Delay 1.0)
            (Variables|Default|SetIs%20open true)))
        (else
          (CallFunction|PrintText (Variables|Default|GetLocked_text) 1))))))

(fn ConstructionScript
  (bind _container_item_model (Variables|Default|GetContainer%20Item%20Model))
  (Utilities|IsValid (Variables|Default|GetSkeletal%20mesh_model)
    (:Is%20Valid
      (Class|SkinnedMeshComponent|SetSkeletalMesh (Variables|Default|GetSkeletalMesh) (Variables|Default|GetSkeletal%20mesh_model) true)
      (Utilities|IsValid _container_item_model
        (:Is%20Valid
          (Components|StaticMesh|SetStaticMesh (Variables|Default|GetContainer_item) _container_item_model))))))

(fn Interaction
  (Components|Animation|PlayAnimation (Variables|Default|GetSkeletalMesh) (Variables|Default|GetOpening%20Animation) false)
  (return))

(fn PickupContainerItem
  (Utilities|IsValid (Variables|Default|GetContainer%20Item%20Model)
    (:Is%20Valid
      (CallFunction|PlayerPickup)
      (CallFunction|PrintText (Variables|Default|GetInteraction_text) 1)
      (Components|DestroyComponent (Variables|Default|GetContainer_item))
      (return))))