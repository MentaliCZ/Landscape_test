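; A weighted pressure button that stays pressed while at least one actor with the allowed tag rests on it.
; Its collision box counts tagged overlaps, calling OnButtonPress on the first arrival and OnButtonOut when the count drops to zero.
; A timeline lerps the button part downward on press and reverses on release.
; The construction script applies configurable base and button meshes.
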(event OnComponentBeginOverlap(Collision_box)
  (params (OverlappedComponent :type Primitive%20Component%20Object%20Reference) (OtherActor :type Actor%20Object%20Reference) (OtherComp :type Primitive%20Component%20Object%20Reference) (OtherBodyIndex :type Integer) (bFromSweep :type Boolean) (SweepResult :type Hit%20Result%20Structure%20%28by%20ref%29))
  (if (Actor|ActorHasTag OtherActor (Variables|Default|GetButton_allowed_tag))
    (Variables|Default|Setnumber_of_objects_on_button (+ (Variables|Default|Getnumber_of_objects_on_button) 1))
    (if (not (Variables|Default|GetPressed))
      (Default|CallOnButtonPress)
      (Variables|Default|SetPressed true)
      (bind _buttonpress (Timeline|ButtonPress_Timeline Play)
        (:Update
          (Transformation|SetRelativeLocation (Variables|Default|GetButton_part) (Math|Vector|MakeVector 0.0 0.0 (Math|Float|Lerp 0.0 (* (Variables|Default|GetButton_pos) -1.0) _buttonpress)) false false))))))

(event OnComponentEndOverlap(Collision_box)
  (params (OverlappedComponent :type Primitive%20Component%20Object%20Reference) (OtherActor :type Actor%20Object%20Reference) (OtherComp :type Primitive%20Component%20Object%20Reference) (OtherBodyIndex :type Integer))
  (if (Actor|ActorHasTag OtherActor (Variables|Default|GetButton_allowed_tag))
    (Variables|Default|Setnumber_of_objects_on_button (- (Variables|Default|Getnumber_of_objects_on_button) 1))
    (if (and (<= (Variables|Default|Getnumber_of_objects_on_button) 0) (Variables|Default|GetPressed))
      (if true
        (Variables|Default|SetPressed false)
        (Default|CallOnButtonOut)
        (bind _buttonpress (Timeline|ButtonPress_Timeline Reverse)
          (:Update
            (Transformation|SetRelativeLocation (Variables|Default|GetButton_part) (Math|Vector|MakeVector 0.0 0.0 (Math|Float|Lerp 0.0 (* (Variables|Default|GetButton_pos) -1.0) _buttonpress)) false false)))))))

(event EventBeginPlay)

(event EventTick
  (params (DeltaSeconds :type Float%20%28single-precision%29)))

(fn ConstructionScript
  (bind _button_base_model (Variables|Default|GetButton_base_model))
  (bind _button_part_model (Variables|Default|GetButton_part_model))
  (Utilities|IsValid _button_base_model
    (:Is%20Valid
      (Components|StaticMesh|SetStaticMesh (Variables|Default|GetButton) _button_base_model)
      (Utilities|IsValid _button_part_model
        (:Is%20Valid
          (Components|StaticMesh|SetStaticMesh (Variables|Default|GetButton_part) _button_part_model))))))