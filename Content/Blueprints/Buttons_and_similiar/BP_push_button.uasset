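; Interactable push button actor that broadcasts an OnButtonPress event dispatcher when Interact is called while it is not already pressed.
; A timeline lowers ButtonPart along local Z by ButtonPos, then after a short delay clears Pressed and reverses to raise it.
; The construction script applies configurable base and button meshes, setting the button mesh only if the base mesh is also valid.
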(event EventBeginPlay)

(event Collision|EventActorBeginOverlap
  (params (OtherActor :type Actor%20Object%20Reference)))

(event EventTick
  (params (DeltaSeconds :type Float%20%28single-precision%29)))

(event EventInteract
  (params (Hit%20Component :type Actor%20Component%20Object%20Reference))
  (if (not (Variables|Default|GetPressed))
    (Default|CallOnButtonPress)
    (Variables|Default|SetPressed true)
    (bind _buttonpress (Timeline|ButtonPress_Timeline PlayFromStart)
      (:Update
        (Transformation|SetRelativeLocation (Variables|Default|GetButton_part) (Math|Vector|MakeVector 0.0 0.0 (Math|Float|Lerp 0.0 (* (Variables|Default|GetButton_pos) -1.0) _buttonpress)) false false))
      (:Finished
        (if (Variables|Default|GetPressed)
          (Utilities|FlowControl|Delay 0.1)
          (Variables|Default|SetPressed false)
          (Timeline|ButtonPress_Timeline ReverseFromEnd))))))

(fn ConstructionScript
  (bind _button_base_model (Variables|Default|GetButton_base_model))
  (bind _button_part_model (Variables|Default|GetButton_part_model))
  (Utilities|IsValid _button_base_model
    (:Is%20Valid
      (Components|StaticMesh|SetStaticMesh (Variables|Default|GetButton) _button_base_model)
      (Utilities|IsValid _button_part_model
        (:Is%20Valid
          (Components|StaticMesh|SetStaticMesh (Variables|Default|GetButton_part) _button_part_model))))))