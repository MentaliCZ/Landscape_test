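; Elevator actor that moves its platform vertically between its base and a set height.
; When set to automatic, the player entering the trigger box raises it after a short delay, and leaving lowers it.
; A single timeline drives the platform's relative Z through a lerp, played forward to rise and reversed to descend.
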(event OnComponentBeginOverlap(Box)
  (params (OverlappedComponent :type Primitive%20Component%20Object%20Reference) (OtherActor :type Actor%20Object%20Reference) (OtherComp :type Primitive%20Component%20Object%20Reference) (OtherBodyIndex :type Integer) (bFromSweep :type Boolean) (SweepResult :type Hit%20Result%20Structure%20%28by%20ref%29))
  ;[1 0.5597 0.4189] Automatic doors logic
  (Utilities|FlowControl|Delay 0.2)
  (if (Variables|Default|GetIsAutomatic)
    (if (Actor|ActorHasTag OtherActor "Player")
      (CallFunction|GoingUp))))

(event OnComponentEndOverlap(Box)
  (params (OverlappedComponent :type Primitive%20Component%20Object%20Reference) (OtherActor :type Actor%20Object%20Reference) (OtherComp :type Primitive%20Component%20Object%20Reference) (OtherBodyIndex :type Integer))
  ;[1 0.5597 0.4189] Automatic doors logic
  (if (Variables|Default|GetIsAutomatic)
    (if (Actor|ActorHasTag OtherActor "Player")
      (CallFunction|GoingDown))))

(event Custom|Going_Up
  (bind _going_up_pos (Timeline|Going_Up_Timeline Play)
    (:Update
      (Transformation|SetRelativeLocation (Variables|Default|GetElevator_platform) (Math|Vector|MakeVector 0.0 0.0 (Math|Float|Lerp 0.0 (Variables|Default|GetElevator_height) _going_up_pos)) false false))))

(event Custom|Going_Down
  (bind _going_up_pos (Timeline|Going_Up_Timeline Reverse)
    (:Update
      (Transformation|SetRelativeLocation (Variables|Default|GetElevator_platform) (Math|Vector|MakeVector 0.0 0.0 (Math|Float|Lerp 0.0 (Variables|Default|GetElevator_height) _going_up_pos)) false false))))

(event EventBeginPlay)

(event Collision|EventActorBeginOverlap
  (params (OtherActor :type Actor%20Object%20Reference)))

(event EventTick
  (params (DeltaSeconds :type Float%20%28single-precision%29)))

(fn ConstructionScript)