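; BP_pickable_item is a pickable world item that reacts when a line trace hits it.
; The construction script applies the StaticMeshModel variable to its mesh when that is valid.
; On TraceLineHit it destroys the mesh, calls PlayerPickup, prints its InteractionText, hides the hint text on the first-person character, then destroys itself.
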(event EventBeginPlay
  (|CallParentFunction) ; This node is disabled and will not be called.\nDrag off pins to build functionality.
)

(event Collision|EventActorBeginOverlap
  (params (OtherActor :type Actor%20Object%20Reference))
  (|CallParentFunction OtherActor) ; This node is disabled and will not be called.\nDrag off pins to build functionality.
)

(event EventTick
  (params (DeltaSeconds :type Float%20%28single-precision%29))
  (|CallParentFunction DeltaSeconds) ; This node is disabled and will not be called.\nDrag off pins to build functionality.
)

(event EventTraceLineHit
  (params (Hit%20Component :type Actor%20Component%20Object%20Reference))
  (Components|DestroyComponent (Variables|Default|GetStaticMesh))
  (CallFunction|PlayerPickup)
  (CallFunction|PrintText (Variables|Default|GetInteraction_text) 1)
  (bind _asbp_first_person_character (Utilities|Casting|CastToBP_FirstPersonCharacter (Game|GetPlayerCharacter 0)))
  (Default|HideHintText _asbp_first_person_character)
  (Actor|DestroyActor))

(fn ConstructionScript
  (bind _static_mesh_model (Variables|Default|GetStatic%20Mesh%20Model))
  (Utilities|IsValid _static_mesh_model
    (:Is%20Valid
      (Components|StaticMesh|SetStaticMesh (Variables|Default|GetStaticMesh) _static_mesh_model))))