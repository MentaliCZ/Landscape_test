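; Key_bp is an interactable key pickup that gives the first-person player item ID 1.
; A box overlap shows its text prompt for Player-tagged actors and updates it again on exit.
; Interact runs once, calling Pickup on the character found by class, then removing the mesh and text.
; A newly created Player_HUD widget shows a pickup message for a few seconds before the actor destroys itself.
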(event OnComponentBeginOverlap(Box)
  (params (OverlappedComponent :type Primitive%20Component%20Object%20Reference) (OtherActor :type Actor%20Object%20Reference) (OtherComp :type Primitive%20Component%20Object%20Reference) (OtherBodyIndex :type Integer) (bFromSweep :type Boolean) (SweepResult :type Hit%20Result%20Structure%20%28by%20ref%29))
  (CallFunction|SetTextVisibility OtherActor))

(event OnComponentEndOverlap(Box)
  (params (OverlappedComponent :type Primitive%20Component%20Object%20Reference) (OtherActor :type Actor%20Object%20Reference) (OtherComp :type Primitive%20Component%20Object%20Reference) (OtherBodyIndex :type Integer))
  (CallFunction|SetTextVisibility))

(event EventBeginPlay)

(event Collision|EventActorBeginOverlap
  (params (OtherActor :type Actor%20Object%20Reference)))

(event EventTick
  (params (DeltaSeconds :type Float%20%28single-precision%29)))

(event EventInteract
  (Utilities|FlowControl|DoOnce false
    (:Completed
      (CallFunction|PlayerPickup)
      (bind _returnvalue (UserInterface|CreateWidget "/Game/Player_HUD.Player_HUD_C"))
      (Variables|/Game/Player_HUD.Player_HUD_C|SetInteraction_text _returnvalue "You got a key, wow!")
      (UserInterface|Viewport|AddtoViewport _returnvalue 0)
      (Components|DestroyComponent (Variables|Default|GetStaticMesh))
      (Utilities|FlowControl|Delay 3.0)
      (Widget|RemovefromParent _returnvalue)
      (Actor|DestroyActor))))

(fn ConstructionScript)

(fn PlayerPickup
  (bind _returnvalue (Actor|GetActorOfClass "/Game/FirstPerson/Blueprints/BP_FirstPersonCharacter.BP_FirstPersonCharacter_C"))
  (bind _output_get (Variables|Default|SetItem_ID 1))
  (Default|Pickup _returnvalue _output_get))

(fn SetTextVisibility
  (params (Other_Actor :type Actor%20Object%20Reference))
  (Rendering|SetVisibility (Variables|Default|GetTextRender) (Actor|ActorHasTag Other_Actor "Player") false))