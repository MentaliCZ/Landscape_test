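; Interactable button actor that broadcasts OnButtonPress and animates its ButtonPart being pushed in and released.
; Interact fires the dispatcher immediately, then two timelines move the part down and back up along local Z, separated by a short delay.
; A Pressed flag blocks re-triggering until the release finishes.
; Movement adds a lerped local offset on every timeline update, so travel accumulates per frame rather than being set absolutely.
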(event EventBeginPlay)

(event Collision|EventActorBeginOverlap
  (params (OtherActor :type Actor%20Object%20Reference)))

(event EventTick
  (params (DeltaSeconds :type Float%20%28single-precision%29)))

(event EventInteract
  (params (Hit%20Component :type Actor%20Component%20Object%20Reference))
  (if (not (Variables|Default|GetPressed))
    (Default|CallOnButtonPress)
    (Variables|Default|SetPressed true)
    (bind _buttonpress (Timeline|ButtonPress_Timeline PlayFromStart)
      (:Update
        (Transformation|AddLocalOffset (Variables|Default|GetButton_part) (Math|Vector|MakeVector 0.0 0.0 (Math|Float|Lerp 0.0 (* (Variables|Default|GetButton_pos) -1.0) _buttonpress)) false false))
      (:Finished
        (Utilities|FlowControl|Delay 0.1)
        (bind _buttonpress_2 (Timeline|ButtonPressOut PlayFromStart)
          (:Update
            (Transformation|AddLocalOffset (Variables|Default|GetButton_part) (Math|Vector|MakeVector 0.0 0.0 (Math|Float|Lerp 0.0 (Variables|Default|GetButton_pos) _buttonpress_2)) false false))
          (:Finished
            (Variables|Default|SetPressed false)))))))

(fn ConstructionScript)