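; BP_Chest is an interactable chest that opens once if the player holds its key.
; On Interact, Playehaskey asks the first-person character via HasItem for a hard-coded key ID.
; With the key, a DoOnce gates the open animation and success message; otherwise a missing-key message shows.
; PrintText creates an Example_widget with the message, which is removed from the screen after a short delay.
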(event EventBeginPlay)

(event Collision|EventActorBeginOverlap
  (params (OtherActor :type Actor%20Object%20Reference)))

(event EventTick
  (params (DeltaSeconds :type Float%20%28single-precision%29)))

(event EventInteract
  (bind _haskey (CallFunction|Playehaskey))
  (if _haskey
    (Utilities|FlowControl|DoOnce false
      (:Completed
        (Components|Animation|PlayAnimation (Variables|Default|GetSkeletalMesh) "/Game/Assets/Old_chest/Chest_2022_Anim.Chest_2022_Anim" false)
        (bind _widget (CallFunction|PrintText "You opened a chest"))))
    (else
      (bind _widget_2 (CallFunction|PrintText "You  dont have a key to open this chest :("))))
  (Utilities|FlowControl|Delay 3.0)
  (Widget|RemovefromParent _widget))

(fn ConstructionScript)

(fn Playehaskey
  (bind _returnvalue (Actor|GetActorOfClass "/Game/FirstPerson/Blueprints/BP_FirstPersonCharacter.BP_FirstPersonCharacter_C"))
  (bind _output_get (Variables|Default|SetKey_ID 1))
  (bind _hasitem (Default|HasItem? _returnvalue _output_get))
  (return _hasitem))

(fn PrintText
  (params (Text :type Text))
  (bind _returnvalue (UserInterface|CreateWidget "/Game/Example_widget.Example_widget_C"))
  (Variables|/Game/Example_widget.Example_widget_C|SetInteraction_text _returnvalue Text)
  (UserInterface|Viewport|AddtoViewport _returnvalue 0)
  (return _returnvalue))