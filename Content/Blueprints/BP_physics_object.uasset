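; BP_physics_object is a configurable physics prop whose mesh, weight and button-pressing ability are set through variables.
; When ObjectModel is valid, the construction script applies it to the Object mesh component and uses Weight as the mass scale.
; Within that same check, CanPressButtons adds a matching name to TagsArray, which then replaces the actor's Tags.
; The event graph has no active logic.
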(event EventBeginPlay)

(event Collision|EventActorBeginOverlap
  (params (OtherActor :type Actor%20Object%20Reference)))

(event EventTick
  (params (DeltaSeconds :type Float%20%28single-precision%29)))

(fn ConstructionScript
  (bind _object_model (Variables|Default|GetObject_model))
  (bind _tags_array (Variables|Default|GetTags_array))
  (Utilities|IsValid _object_model
    (:Is%20Valid
      (Components|StaticMesh|SetStaticMesh (Variables|Default|GetObject) _object_model)
      (Class|PrimitiveComponent|SetMassScale (Variables|Default|GetObject) "None" (Math|Conversions|ToFloat(Integer) (Variables|Default|GetWeight)))
      (if (Variables|Default|GetCan%20Press%20Buttons)
        (Utilities|Array|Add _tags_array "CanPressButtons")
        (Variables|Default|SetTags _tags_array)))))