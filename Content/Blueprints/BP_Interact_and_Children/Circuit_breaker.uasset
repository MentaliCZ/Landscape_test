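; Interactable circuit breaker with a countdown, apparently one of several levers that must all be pulled before time runs out.
; Interact animates the lever down, calls LeverPressed and switches a shared dynamic material from red to green.
; Timer counts down each second on a widget display, then reverses a pressed lever, calls LeverOff and restores red.
; All_levers_pull zeroes the display and locks the lever, blocking further interaction and resets.
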(event Custom|Timer
  (if (not (Variables|Default|GetAll_levers_pulled))
    (bind _output_get (Variables|Default|Setdelay (Variables|Default|GetDelay_time)))
    (CallFunction|TextRenderLogic _output_get)
    (if (or (<= (Variables|Default|Getdelay) 0) (Variables|Default|GetAll_levers_pulled)) :!label _label
      (CallFunction|TextRenderLogic)
      (if (and (not (Variables|Default|GetAll_levers_pulled)) (Variables|Default|GetIs%20Pressed))
        (bind _lever_rotation (Timeline|Lever_reverse_timeline ReverseFromEnd)
          (:Update
            (Transformation|SetRelativeRotation (Variables|Default|GetCircuit_breaker_lever) (Math|Rotator|MakeRotator 0.0 (Math|Float|Lerp 0.0 -1.8e+02 _lever_rotation) 0.0) false false))
          (:Finished
            (Default|CallLeverOff)
            (CallFunction|RedLighton)
            (Variables|Default|SetIs%20Pressed false))))
      (else
        (Utilities|FlowControl|Delay 1.0)
        (CallFunction|TextRenderLogic (- (Variables|Default|Getdelay) 1))
        (goto _label)))))

(event Custom|All_levers_pull
  (CallFunction|TextRenderLogic)
  (Variables|Default|SetAll_levers_pulled true)
  (Variables|Default|SetIs%20Pressed true))

(event EventBeginPlay
  ;[1 0.3075 0.3872] Init
  (bind _ascircuit_breaker_timer (Utilities|Casting|CastToCircuit_breaker_timer (UserInterface|GetWidget (Variables|Default|GetWidget))))
  (Variables|Default|SetTimer_widget _ascircuit_breaker_timer)
  (bind _returnvalue (Rendering|Material|CreateDynamicMaterialInstance "/Game/Assets/Circuit_breaker/Circuit_breaker_material.Circuit_breaker_material" "None" "None" :!class /Script/Engine.KismetMaterialLibrary))
  (bind _output_get (Variables|Default|SetMaterial _returnvalue))
  (Rendering|Material|SetMaterial (Variables|Default|GetCircuit_breaker_lever) 0 _output_get)
  (CallFunction|RedLighton)
  (CallFunction|TextRenderLogic))

(event EventInteract
  (params (Hit%20Component :type Actor%20Component%20Object%20Reference))
  (if (not (Variables|Default|GetIs%20Pressed))
    (Variables|Default|SetIs%20Pressed true)
    (bind _lever_rotation (Timeline|Lever_timeline PlayFromStart)
      (:Update
        (Transformation|SetRelativeRotation (Variables|Default|GetCircuit_breaker_lever) (Math|Rotator|MakeRotator 0.0 (Math|Float|Lerp 0.0 -1.8e+02 _lever_rotation) 0.0) false false))
      (:Finished
        (Default|CallLeverPressed)
        (CallFunction|GreenLighton)))))

(fn ConstructionScript)

(fn RedLighton
  (bind _material (Variables|Default|GetMaterial))
  (Rendering|Material|SetScalarParameterValue _material "Green_strength" 0.0 :!class /Script/Engine.MaterialInstanceDynamic)
  (Rendering|Material|SetScalarParameterValue _material "Red_strength" 1.0 :!class /Script/Engine.MaterialInstanceDynamic))

(fn GreenLighton
  (bind _material (Variables|Default|GetMaterial))
  (Rendering|Material|SetScalarParameterValue _material "Green_strength" 1.0 :!class /Script/Engine.MaterialInstanceDynamic)
  (Rendering|Material|SetScalarParameterValue _material "Red_strength" 0.0 :!class /Script/Engine.MaterialInstanceDynamic))

(fn TextRenderLogic
  (params (Seconds :type Integer))
  (bind _returnvalue (Utilities|Text|ToText(Integer) Seconds))
  (bind _returnvalue_2 (Utilities|String|ToString(Text) _returnvalue))
  (bind _output_get (Variables|Default|Setdelay Seconds))
  (if (<= _output_get 9)
    (Variables|/Game/Assets/Circuit_breaker/Circuit_breaker_timer.Circuit_breaker_timer_C|SetTimer_text (Variables|Default|GetTimer_widget) (Utilities|Text|ToText(String) (Utilities|String|Append "0:0" _returnvalue_2)))
    (else
      (Variables|/Game/Assets/Circuit_breaker/Circuit_breaker_timer.Circuit_breaker_timer_C|SetTimer_text (Variables|Default|GetTimer_widget) (Utilities|Text|ToText(String) (Utilities|String|Append "0:" _returnvalue_2))))))