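; Interactable door Blueprint that swings open and closed on alternate interactions, or prints locked text when it is not unlocked.
; A timeline lerps the yaw of both static and skeletal door components to 90 degrees, reversing to close.
; Without a static door model, each toggle also plays the skeletal opening animation.
; The construction script applies the frame mesh, then a static or fallback skeletal door mesh, only if a frame model is set.
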(event EventBeginPlay)

(event Collision|EventActorBeginOverlap
  (params (OtherActor :type Actor%20Object%20Reference)))

(event EventInteract
  (params (Hit%20Component :type Actor%20Component%20Object%20Reference))
  (bind _isunlocked (CallFunction|IsUnlocked))
  (if _isunlocked
    (Utilities|FlowControl|FlipFlop
      (:A
        (CallFunction|SkeletalDoorLogic)
        (bind _door_open (Timeline|Open_door_timeline PlayFromStart)
          (:Update
            (Transformation|SetRelativeRotation (Variables|Default|GetDoor) (Math|Rotator|MakeRotator 0.0 0.0 (Math|Float|Lerp 0.0 9e+01 _door_open)) false false))))
      (:B
        (CallFunction|SkeletalDoorLogic)
        (Timeline|Open_door_timeline ReverseFromEnd)))
    (else
      (CallFunction|PrintText (Variables|Default|GetLocked_text) 1))))

(fn ConstructionScript
  (bind _doorframe_model (Variables|Default|GetDoorFrame_model))
  (bind _door_model (Variables|Default|GetDoor_model))
  (bind _doorskeletal_model (Variables|Default|GetDoorSkeletal_model))
  (Utilities|IsValid _doorframe_model
    (:Is%20Valid
      (Components|StaticMesh|SetStaticMesh (Variables|Default|GetDoorFrame) _doorframe_model)
      (Utilities|IsValid _door_model
        (:Is%20Valid
          (Components|StaticMesh|SetStaticMesh (Variables|Default|GetDoor) _door_model))
        (:Is%20Not%20Valid
          (Utilities|IsValid _doorskeletal_model
            (:Is%20Valid
              (Components|SkeletalMesh|SetSkeletalMeshAsset (Variables|Default|GetDoor_skeletal) _doorskeletal_model))))))))

(fn SkeletalDoorLogic
  (bind _opening_animation (Variables|Default|GetOpening_animation))
  (Utilities|IsValid (Variables|Default|GetDoor_model)
    (:Is%20Not%20Valid
      (Utilities|IsValid _opening_animation
        (:Is%20Valid
          (Components|Animation|PlayAnimation (Variables|Default|GetDoor_skeletal) _opening_animation false))))))