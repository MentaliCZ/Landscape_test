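; BP_InteractableItem is an interactable item that shows the player a hint when nearby and can be picked up.
; When a Player-tagged actor enters its Box, it prints HintText and polls a PlayerCollision flag in a short Delay loop until the overlap ends, then calls HideHintText on the first-person character.
; PlayerPickup passes the item's ItemID to BP_FirstPersonCharacter's Pickup.
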(event OnComponentBeginOverlap(Box)
  (params (OverlappedComponent :type Primitive%20Component%20Object%20Reference) (OtherActor :type Actor%20Object%20Reference) (OtherComp :type Primitive%20Component%20Object%20Reference) (OtherBodyIndex :type Integer) (bFromSweep :type Boolean) (SweepResult :type Hit%20Result%20Structure%20%28by%20ref%29))
  ;[1 0.5103 0.1612] Show Hints
  (if (Actor|ActorHasTag OtherActor "Player")
    (CallFunction|PrintText (Variables|Default|GetHint%20Text) 2)
    (bind _output_get (Variables|Default|SetPlayer_collision true))
    (if _output_get :!label _label
      (Utilities|FlowControl|Delay 0.2)
      (goto _label)
      (else
        (bind _asbp_first_person_character (Utilities|Casting|CastToBP_FirstPersonCharacter (Game|GetPlayerCharacter 0)))
        (Default|HideHintText _asbp_first_person_character)))))

(event OnComponentEndOverlap(Box)
  (params (OverlappedComponent :type Primitive%20Component%20Object%20Reference) (OtherActor :type Actor%20Object%20Reference) (OtherComp :type Primitive%20Component%20Object%20Reference) (OtherBodyIndex :type Integer))
  ;[1 0.5103 0.1612] Show Hints
  (Variables|Default|SetPlayer_collision false))

(event EventBeginPlay)

(event Collision|EventActorBeginOverlap
  (params (OtherActor :type Actor%20Object%20Reference)))

(event EventTick
  (params (DeltaSeconds :type Float%20%28single-precision%29)))

(fn ConstructionScript)

(fn PlayerPickup
  ;[1 1 1] Player Pickup
  (bind _returnvalue (Actor|GetActorOfClass "/Game/FirstPerson/Blueprints/BP_FirstPersonCharacter.BP_FirstPersonCharacter_C"))
  (Default|Pickup _returnvalue (Variables|Default|GetItem%20ID)))