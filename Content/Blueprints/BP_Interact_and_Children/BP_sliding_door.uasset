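; Two-panel sliding door that opens and closes via Open and Close events, or automatically for actors tagged Player when IsAutomatic is set.
; A timeline plays forward or in reverse, driving a lerp that moves the panels in opposite directions along local Y.
; Collision box begin and end overlaps trigger the automatic mode.
; The construction script applies configurable frame and panel meshes, each nested on the previous one being valid.
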(event OnComponentBeginOverlap(CollisionBox)
  (params (OverlappedComponent :type Primitive%20Component%20Object%20Reference) (OtherActor :type Actor%20Object%20Reference) (OtherComp :type Primitive%20Component%20Object%20Reference) (OtherBodyIndex :type Integer) (bFromSweep :type Boolean) (SweepResult :type Hit%20Result%20Structure%20%28by%20ref%29))
  ;[1 0.5597 0.4189] Automatic doors logic
  (if (Variables|Default|GetIsAutomatic)
    (if (Actor|ActorHasTag OtherActor "Player")
      (CallFunction|Open))))

(event OnComponentEndOverlap(CollisionBox)
  (params (OverlappedComponent :type Primitive%20Component%20Object%20Reference) (OtherActor :type Actor%20Object%20Reference) (OtherComp :type Primitive%20Component%20Object%20Reference) (OtherBodyIndex :type Integer))
  ;[1 0.5597 0.4189] Automatic doors logic
  (if (Variables|Default|GetIsAutomatic)
    (if (Actor|ActorHasTag OtherActor "Player")
      (CallFunction|Close))))

(event Custom|Open
  ;[0.5153 0.9301 1] Open and Close
  (Variables|Default|SetIsOpen true)
  (bind _sliding_door_open (Timeline|Sliding_door_open Play)
    (:Update
      (Transformation|SetRelativeLocation (Variables|Default|GetLeft_door) (Math|Vector|MakeVector 0.0 (Math|Float|Lerp 0.0 (Variables|Default|GetB) _sliding_door_open) 0.0) false false)
      (Transformation|SetRelativeLocation (Variables|Default|GetRight_door) (Math|Vector|MakeVector 0.0 (* (Math|Float|Lerp 0.0 (Variables|Default|GetB) _sliding_door_open) -1.0) 0.0) false false))))

(event Custom|Close
  ;[0.5153 0.9301 1] Open and Close
  (Variables|Default|SetIsOpen false)
  (bind _sliding_door_open (Timeline|Sliding_door_open Reverse)
    (:Update
      (Transformation|SetRelativeLocation (Variables|Default|GetLeft_door) (Math|Vector|MakeVector 0.0 (Math|Float|Lerp 0.0 (Variables|Default|GetB) _sliding_door_open) 0.0) false false)
      (Transformation|SetRelativeLocation (Variables|Default|GetRight_door) (Math|Vector|MakeVector 0.0 (* (Math|Float|Lerp 0.0 (Variables|Default|GetB) _sliding_door_open) -1.0) 0.0) false false))))

(event EventBeginPlay)

(event Collision|EventActorBeginOverlap
  (params (OtherActor :type Actor%20Object%20Reference)))

(event EventTick
  (params (DeltaSeconds :type Float%20%28single-precision%29)))

(fn ConstructionScript
  (bind _door_frame_model (Variables|Default|GetDoor_frame_model))
  (bind _left_door_model (Variables|Default|GetLeft_door_model))
  (bind _right_door_model (Variables|Default|GetRight_door_model))
  (Utilities|IsValid _door_frame_model
    (:Is%20Valid
      (Components|StaticMesh|SetStaticMesh (Variables|Default|GetDoor_frame) _door_frame_model)
      (Utilities|IsValid _left_door_model
        (:Is%20Valid
          (Components|StaticMesh|SetStaticMesh (Variables|Default|GetLeft_door) _left_door_model)
          (Utilities|IsValid _right_door_model
            (:Is%20Valid
              (Components|StaticMesh|SetStaticMesh (Variables|Default|GetRight_door) _right_door_model))))))))