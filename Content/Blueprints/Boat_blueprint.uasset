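; Boat escape objective: the player loads a plastic barrel, canteen and lifebuoy, then interacts to show the ending HUD.
; Tagged physics items overlapping the deck are matched by ID, destroyed, and replaced by pre-placed hidden meshes, whose visibility doubles as progress state.
; A hint text, shown while the player is inside the box trigger and rotated each tick using camera position, is rebuilt from the missing items.
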(event OnComponentBeginOverlap(Box)
  (params (OverlappedComponent :type Primitive%20Component%20Object%20Reference) (OtherActor :type Actor%20Object%20Reference) (OtherComp :type Primitive%20Component%20Object%20Reference) (OtherBodyIndex :type Integer) (bFromSweep :type Boolean) (SweepResult :type Hit%20Result%20Structure%20%28by%20ref%29))
  (if (Actor|ActorHasTag OtherActor "Player")
    (Rendering|SetVisibility (Variables|Default|GetHint_text) true false)))

(event OnComponentEndOverlap(Box)
  (params (OverlappedComponent :type Primitive%20Component%20Object%20Reference) (OtherActor :type Actor%20Object%20Reference) (OtherComp :type Primitive%20Component%20Object%20Reference) (OtherBodyIndex :type Integer))
  (if (Actor|ActorHasTag OtherActor "Player")
    (Rendering|SetVisibility (Variables|Default|GetHint_text) false false)))

(event OnComponentBeginOverlap(Deck_collider)
  (params (OverlappedComponent :type Primitive%20Component%20Object%20Reference) (OtherActor :type Actor%20Object%20Reference) (OtherComp :type Primitive%20Component%20Object%20Reference) (OtherBodyIndex :type Integer) (bFromSweep :type Boolean) (SweepResult :type Hit%20Result%20Structure%20%28by%20ref%29))
  (if (Actor|ActorHasTag OtherActor "CanBePlacedOnBoat")
    (bind _asbp_physics_object (Utilities|Casting|CastToBP_physics_object OtherActor))
    (switch int (Variables|/Game/Blueprints/BP_physics_object.BP_physics_object_C|GetBoat_item_ID _asbp_physics_object)
      (:0
        (CallFunction|ItemonBoardLogic "The plastic barrel is on board" (Variables|Default|GetPlastic%20Barrel)))
      (:1
        (CallFunction|ItemonBoardLogic "The canteen is on board" (Variables|Default|GetCanteen)))
      (:2
        (CallFunction|ItemonBoardLogic "The lifebuoy is on board" (Variables|Default|GetLifeBuoy))))
    (Actor|DestroyActor _asbp_physics_object)))

(event EventTick
  (params (DeltaSeconds :type Float%20%28single-precision%29))
  (Transformation|SetWorldRotation (Variables|Default|GetHint_text) (Math|Rotator|MakeRotfromX (- (Transformation|GetWorldLocation (Variables|Default|GetHint_text)) (Transformation|GetActorLocation (Game|GetPlayerCameraManager 0)))) false false))

(event EventInteract
  (params (Hit%20Component :type Actor%20Component%20Object%20Reference))
  (if (and (and (Rendering|IsVisible (Variables|Default|GetCanteen)) (Rendering|IsVisible (Variables|Default|GetLifeBuoy))) (Rendering|IsVisible (Variables|Default|GetPlastic%20Barrel)))
    (CallFunction|EndingSequence)))

(fn ConstructionScript
  (Rendering|SetVisibility (Variables|Default|GetLifeBuoy) false false)
  (CallFunction|HintTextLogic)
  (Rendering|SetVisibility (Variables|Default|GetHint_text) false false))

(fn ItemonBoardLogic
  (params (Interaction_text :type Text) (Object_ref :type Scene%20Component%20Object%20Reference))
  (bind _output_get (Variables|Default|SetInteraction_text Interaction_text))
  (CallFunction|PrintText _output_get 1)
  (Rendering|SetVisibility Object_ref true false)
  (CallFunction|HintTextLogic))

(fn HintTextLogic
  (Variables|Default|SetHint_text_renderer "You need")
  (if (not (Rendering|IsVisible (Variables|Default|GetCanteen)))
    (Variables|Default|SetHint_text_renderer (Utilities|Text|ToText(String) (Utilities|String|Append (Utilities|String|ToString(Text) (Variables|Default|GetHint_text_renderer)) (Utilities|String|Append "<br>" "Water Canteen")))))
  (if (not (Rendering|IsVisible (Variables|Default|GetLifeBuoy)))
    (Variables|Default|SetHint_text_renderer (Utilities|Text|ToText(String) (Utilities|String|Append (Utilities|String|ToString(Text) (Variables|Default|GetHint_text_renderer)) (Utilities|String|Append "<br>" "Life Buoy")))))
  (if (not (Rendering|IsVisible (Variables|Default|GetPlastic%20Barrel)))
    (Variables|Default|SetHint_text_renderer (Utilities|Text|ToText(String) (Utilities|String|Append (Utilities|String|ToString(Text) (Variables|Default|GetHint_text_renderer)) (Utilities|String|Append "<br>" "Plastic Barrel"))))
    (elif (and (Rendering|IsVisible (Variables|Default|GetCanteen)) (and (Rendering|IsVisible (Variables|Default|GetPlastic%20Barrel)) (Rendering|IsVisible (Variables|Default|GetLifeBuoy))))
      (Variables|Default|SetHint_text_renderer "")
      (Variables|Default|SetHint%20Text "Press E to leave")))
  (Rendering|Components|TextRender|SetText (Variables|Default|GetHint_text) (Variables|Default|GetHint_text_renderer)))

(fn EndingSequence
  (bind _returnvalue (UserInterface|CreateWidget "/Game/Widgets/Ending_HUD.Ending_HUD_C"))
  (UserInterface|Viewport|AddtoViewport _returnvalue 0))